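; BP_GameBlock is a track block with lanes, apparently one segment of a runner course extended by the game mode.
; On OverlapBox overlap it waits and destroys itself before the character check, so any overlapping actor triggers removal.
; The following character-only steps call AddGameBlock on BP_ThirdPersonGameMode, then repeat the delayed destroy.
; BeginPlay enables collision on Lane1, Lane2 and Lane4, while the Lane3 call is disconnected.
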(event `self.OverlapBox.OnComponentBeginOverlap`
  (params (OverlappedComponent :type "PrimitiveComponent Object Reference") (OtherActor :type "Actor Object Reference") (OtherComp :type "PrimitiveComponent Object Reference") (OtherBodyIndex :type Integer) (bFromSweep :type Boolean) (SweepResult :type "HitResult Structure (by ref)"))
  (`KismetSystemLibrary.Delay` 5.0)
  (`self.K2_DestroyActor`)
  (cast `/Game/ThirdPerson/Blueprints/BP_ThirdPersonCharacter` OtherActor)
  (bind _asbp_third_person_game_mode (cast `/Game/ThirdPerson/Blueprints/BP_ThirdPersonGameMode` (`GameplayStatics.GetGameMode`)))
  (`/Game/ThirdPerson/Blueprints/BP_ThirdPersonGameMode.AddGameBlock` _asbp_third_person_game_mode)
  (`KismetSystemLibrary.Delay` 5.0)
  (`self.K2_DestroyActor`))

(event `self.ReceiveBeginPlay`
  (`PrimitiveComponent.SetCollisionEnabled` (`self.Lane1`) "QueryAndPhysics")
  (`PrimitiveComponent.SetCollisionEnabled` (`self.Lane2`) "QueryAndPhysics")
  (`PrimitiveComponent.SetCollisionEnabled` (`self.Lane4`) "QueryAndPhysics"))

(fn `UserConstructionScript`)